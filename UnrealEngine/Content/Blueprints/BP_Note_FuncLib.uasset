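; Blueprint function library of lookup helpers for notes and their judgement, apparently for a rhythm game.
; Key helpers map numpad 1-9 to a 3x3 Horizontal/Vertical coordinate and arrow keys to directions, defaulting to NumPad 1's cell and Up.
; Direction helpers convert a direction into an angle or a rotation.
; GetJudgeEffect picks the Niagara effect for a Perfect or Good result.
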(fn GetJudgeEffect
  (params (result :type JudgeResult%20Enum :default "perfect"))
  (switch Utilities|FlowControl|Switch|SwitchonJudgeResult result
    (:perfect
      (return "/Game/VFX_Niagara/NS_Perfect_Judge.NS_Perfect_Judge"))
    (:good
      (return "/Game/VFX_Niagara/NS_Good_Judge.NS_Good_Judge"))))

(fn GetDirectionAngle
  (params (direction :type NoteDirection%20Enum :default "none"))
  (switch Utilities|FlowControl|Switch|SwitchonNoteDirection direction
    (:none
      _)
    (:left
      (return 9e+01))
    (:right
      (return -9e+01))
    (:up
      _)
    (:down
      (return 1.8e+02)))
  (return 0.0))

(fn GetCoordinatefromKey
  (params (input%20key :type Key%20Structure :default "None"))
  (if (== input%20key "NumPadOne")
    _
    (elif (== input%20key "NumPadTwo")
      (return "right" "middle")
      (elif (== input%20key "NumPadThree")
        (return "right" "right")
        (elif (== input%20key "NumPadFour")
          (return "middle" "left")
          (elif (== input%20key "NumPadFive")
            (return "middle" "middle")
            (elif (== input%20key "NumPadSix")
              (return "middle" "right")
              (elif (== input%20key "NumPadSeven")
                (return "left" "left")
                (elif (== input%20key "NumPadEight")
                  (return "left" "middle")
                  (elif (== input%20key "NumPadNine")
                    (return "left" "right")
                    (else
                      _))))))))))
  (return "right" "left"))

(fn GetDirectionfromKey
  (params (input%20key :type Key%20Structure :default "None"))
  (if (== input%20key "Up")
    _
    (elif (== input%20key "Down")
      (return "down")
      (elif (== input%20key "Left")
        (return "left")
        (elif (== input%20key "Right")
          (return "right")
          (else
            _)))))
  (return "up"))

(fn GetDirectionRotation
  (params (direction :type NoteDirection%20Enum :default "none"))
  (switch Utilities|FlowControl|Switch|SwitchonNoteDirection direction
    (:left
      (return "0,90.000000, 0"))
    (:right
      (return "0,-90.000000, 0"))
    (:up
      (return "-90.000000,0.000000, 0"))
    (:down
      (return "90.000000, 0, 0"))))