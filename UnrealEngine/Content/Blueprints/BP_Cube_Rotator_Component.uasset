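; Actor component that rotates its owner in a set Direction over a limited Duration, then destroys itself.
; BeginPlay resets the remaining time to Duration.
; Each Tick applies the direction's rotation in local space, scaled by the whole-number quotient of the time step over Duration.
; The final step uses only the leftover time before the component is destroyed.
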(event EventTick
  (params (DeltaSeconds :type Float%20%28single-precision%29))
  (Variables|Default|SetDelta%20Seconds DeltaSeconds)
  (Variables|Default|Setcontinue (> (Variables|Default|Getremaining) (Variables|Default|GetDelta%20Seconds)))
  (Transformation|AddActorLocalRotation (Components|GetOwner) (* (CallFunction|GetDirectionRotation (Variables|Default|Getdirection)) (.ReturnValue (Math|Float|Division(WholeandRemainder) (select (Variables|Default|Getcontinue) (Variables|Default|GetDelta%20Seconds) (Variables|Default|Getremaining)) (Variables|Default|Getduration)))) false false)
  (if (Variables|Default|Getcontinue)
    (Variables|Default|Setremaining (- (Variables|Default|Getremaining) (Variables|Default|GetDelta%20Seconds)))
    (else
      (Components|DestroyComponent))))

(event EventBeginPlay
  (CallFunction|Reset))

(fn Reset
  (Variables|Default|Setremaining (Variables|Default|Getduration)))