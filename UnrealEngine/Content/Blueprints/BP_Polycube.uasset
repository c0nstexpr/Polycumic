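; Main actor of a cube-based rhythm game, linking the menu widget, imported audio and note system.
; Import loads a picked audio file at runtime plus the chart.json beside it; UI buttons control playback, tick and input.
; Audio playback time clocks note updates and judgement.
; Direction keys rotate the cube and note system, and note keys submit grid coordinate, direction and surface for judging.
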(event EventBeginPlay
  (bind _returnvalue (UserInterface|CreateWidget "/Game/Blueprints/BP_Main_Widget.BP_Main_Widget_C"))
  (UserInterface|Viewport|AddtoViewport _returnvalue 0)
  (Variables|/Script/Engine.PlayerController|SetbShowMouseCursor (Game|GetPlayerController 0) true)
  (|BindUI _returnvalue))

(event EventTick
  (params (DeltaSeconds :type Float%20%28single-precision%29))
  (Class|NoteSystem|Update (Variables|Default|GetBP_NoteSystem) (CallFunction|GetPlayTime)))

(event Input|ActionEvents|InputActionNote
  (params (Key :type Key%20Structure))
  (bind (_horizontal _vertical) (CallFunction|GetCoordinatefromKey Key))
  (:Pressed
    (Class|NoteSystem|JudgeInput (Variables|Default|GetBP_NoteSystem) _horizontal _vertical (Variables|Default|Getinput%20direction) (Variables|Default|Getsurface) (CallFunction|GetPlayTime))
    (Variables|Default|Setinput%20direction "none")))

(event Input|ActionEvents|InputActionDirection
  (params (Key :type Key%20Structure))
  (:Pressed
    (bind _output_get (Variables|Default|Setinput%20direction (CallFunction|GetDirectionfromKey Key)))
    (CallFunction|Rotate _output_get))
  (:Released
    (Variables|Default|Setinput%20direction "none")))

(fn ConstructionScript)

(fn Rotate
  (params (direction :type NoteDirection%20Enum :default "none"))
  (if (Utilities|Enum|NotEqual(Enum) direction "none")
    (AddComponent|AddBPCubeRotatorComponent direction 0.5 (Variables|Default|GetSM_Polycube))
    (Class|NoteSystem|Rotate (Variables|Default|GetBP_NoteSystem) direction)))

(fn GetPlayTime
  (return (Class|ImportedSoundWave|GetPlaybackTime (Variables|Default|Getsound%20wave%20ref))))

(fn ClearAudio
  (Audio|Components|Audio|SetSound (Variables|Default|GetAudio) 0)
  (Utilities|IsValid (Variables|Default|Getsound%20wave%20ref)
    (:Is%20Valid
      (Class|ImportedSoundWave|ReleaseMemory (Variables|Default|Getsound%20wave%20ref)))
    (:Is%20Not%20Valid
      _))
  (Variables|Default|Setsound%20wave%20ref 0))

(fn IsLoaded
  (return (and (Utilities|IsValid (Variables|/Script/Engine.AudioComponent|GetSound (Variables|Default|GetAudio))) (Class|NoteSystem|IsLoaded (Variables|Default|GetBP_NoteSystem)))))

(event Custom|On%20Import
  (if (not (Variables|Default|Getis%20importing))
    (Variables|Default|Setis%20importing true)
    (bind (_outfilenames _returnvalue) (Class|EFDFunctionLibrary|OpenFileDialog "Import Chart From Aduio" "" "" "" "Single"))
    (Variables|Default|Setis%20importing false)
    (if _returnvalue
      (bind _returnvalue_2 (Class|RuntimeAudioImporterLibrary|CreateRuntimeAudioImporter))
      (EventDispatchers|BindEventtoOnResult _returnvalue_2 (delegate OnImportedAudioDef))
      (Class|RuntimeAudioImporterLibrary|ImportAudiofromFile _returnvalue_2 (Utilities|Array|Get(acopy) _outfilenames) "Auto")
      (Class|NoteSystem|LoadChartPath (Variables|Default|GetBP_NoteSystem) (Class|BlueprintPathsLibrary|Combine (Utilities|Array|MakeArray (Class|FileSystemFuncLib|GetDirectory (Utilities|Array|Get(acopy) _outfilenames)) "chart.json"))))))

(event Custom|On%20Imported%20Audio
  (params (RuntimeAudioImporterObjectRef :type Runtime%20Audio%20Importer%20Library%20Object%20Reference) (SoundWaveRef :type Imported%20Sound%20Wave%20Object%20Reference) (Status :type ETranscodingStatus%20Enum%20%28by%20ref%29 :default "SuccessImporting"))
  (bind _audio (Variables|Default|GetAudio))
  (CallFunction|ClearAudio)
  (switch Utilities|FlowControl|Switch|SwitchonETranscodingStatus Status
    (:SuccessImporting
      (bind _output_get (Variables|Default|Setsound%20wave%20ref SoundWaveRef))
      (Audio|Components|Audio|SetSound _audio _output_get)
      (Audio|Components|Audio|Play _audio 0.0)
      (Class|AudioComponent|SetPaused _audio true))))

(event Custom|On%20Play
  (if (CallFunction|IsLoaded)
    (Input|EnableInput (Game|GetPlayerController 0))
    (Class|AudioComponent|SetPaused (Variables|Default|GetAudio) false)
    (Actor|Tick|SetActorTickEnabled true)))

(event Custom|Event%20Reaction%20Time%20Changed
  (params (time :type Float%20%28single-precision%29))
  (Class|NoteSystem|SetReactionTime (Variables|Default|GetBP_NoteSystem) time))

(event Custom|Event%20Stop
  (Class|AudioComponent|SetPaused (Variables|Default|GetAudio) true)
  (Actor|Tick|SetActorTickEnabled false)
  (Input|DisableInput (Game|GetPlayerController 0)))

(event Custom|On%20Retry
  (if (CallFunction|IsLoaded)
    (if (Audio|Components|Audio|IsPlaying (Variables|Default|GetAudio))
      (Class|ImportedSoundWave|RewindPlaybackTime (Variables|Default|Getsound%20wave%20ref) 0.0))
    (Class|NoteSystem|Reload (Variables|Default|GetBP_NoteSystem))
    (CallFunction|EventStop)))