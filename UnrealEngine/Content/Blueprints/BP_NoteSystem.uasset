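; BP_NoteSystem is a component that spawns notes and relays judgement results to them, apparently for a rhythm game.
; It caches its owner on BeginPlay, and Instantiate spawns a BP_Note or, when given a direction, a BP_Directional_Note at the owner's transform.
; Each new note is snap-attached to the owner and returned.
; PerformJudgeRes casts the given note to BP_Note and triggers its judge effect with the result.
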(event EventBeginPlay
  (Variables|Default|Setparent (Components|GetOwner)))

(event EventPerformJudgeRes
  (params (note :type Actor%20Object%20Reference) (result :type JudgeResult%20Enum :default "perfect"))
  (bind _asbp_note (Utilities|Casting|CastToBP_Note note))
  (Default|PerformJudgeEffect _asbp_note result))

(fn Instantiate
  (params (direction :type NoteDirection%20Enum :default "none"))
  (bind _parent (Variables|Default|Getparent))
  (bind _returnvalue (Transformation|GetActorTransform _parent))
  (if (Utilities|Enum|Equal(Enum) direction "none")
    (bind _returnvalue_2 (Game|SpawnActorfromClass "/Game/Blueprints/BP_Note.BP_Note_C" _returnvalue "Undefined" 0 0))
    (LocalVariables|Setinstance _returnvalue_2)
    (else
      (bind _returnvalue_3 (Game|SpawnActorfromClass "/Game/Blueprints/BP_Directional_Note.BP_Directional_Note_C" _returnvalue "Undefined" 0 direction 0))
      (LocalVariables|Setinstance _returnvalue_3)))
  (Transformation|AttachActorToActor (LocalVariables|Getinstance) (Variables|Default|Getparent) "None" "SnapToTarget" "SnapToTarget" "SnapToTarget" true)
  (return (LocalVariables|Getinstance)))